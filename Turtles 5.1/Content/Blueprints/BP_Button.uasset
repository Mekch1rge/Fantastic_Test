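; BP_Button is an interactable numbered button that plays a sound and fires a spawn dispatcher with its index when used.
; On BeginPlay it derives that index from its position in the GetAllActorsOfClass result, so numbering follows that array's order, and displays it one-based.
; A box overlap shows the Helper component while BP_Player is inside and hides it on exit.
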(event `/Game/Blueprints/BP_Interact_Interface.Interact`
  (`GameplayStatics.PlaySound2D` "/Game/Sounds/SC_RandomInteraction.SC_RandomInteraction" 1.0 1.0 0.0 null null)
  (`self.Spawn_Dispatcher` (`self.Index`)))

(event `self.ReceiveBeginPlay`
  (`self.SetIndex`)
  (`TextRenderComponent.K2_SetText` (`self.Name`) (`KismetTextLibrary.Conv_IntToText` (+ (`self.Index`) 1))))

(event `self.Box.OnComponentBeginOverlap`
  (params (OverlappedComponent :type "PrimitiveComponent Object Reference") (OtherActor :type "Actor Object Reference") (OtherComp :type "PrimitiveComponent Object Reference") (OtherBodyIndex :type Integer) (bFromSweep :type Boolean) (SweepResult :type "HitResult Structure (by ref)"))
  (cast `/Game/Blueprints/BP_Player` OtherActor)
  (`SceneComponent.SetHiddenInGame` (`self.Helper`) false false))

(event `self.Box.OnComponentEndOverlap`
  (params (OverlappedComponent :type "PrimitiveComponent Object Reference") (OtherActor :type "Actor Object Reference") (OtherComp :type "PrimitiveComponent Object Reference") (OtherBodyIndex :type Integer))
  (cast `/Game/Blueprints/BP_Player` OtherActor)
  (`SceneComponent.SetHiddenInGame` (`self.Helper`) true false))

(fn `SetIndex`
  (bind _outactors (`GameplayStatics.GetAllActorsOfClass` "BP_Button_C"))
  (for (_array_element _array_index) _outactors
    (if (== _array_element self)
      (break)))
  (set `self.Index` _array_index))

(fn `UserConstructionScript`)